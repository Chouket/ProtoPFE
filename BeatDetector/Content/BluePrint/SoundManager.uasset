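; SoundManager is an actor Blueprint that connects an FMOD audio component, FMODAudioScene, to the user interface.
; On BeginPlay, InitUI creates a UserUI widget, hands it the audio component and shows it.
; The component's timeline beat and marker callbacks only print debug strings.
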(event `self.ReceiveBeginPlay`
  (`self.InitUI`))

(event `self.ReceiveTick`
  (params (DeltaSeconds :type "Float (single-precision)")))

(event `self.FMODAudioScene.OnTimelineBeat`
  (params (Bar :type Integer) (Beat :type Integer) (Position :type Integer) (Tempo :type "Float (single-precision)") (TimeSignatureUpper :type Integer) (TimeSignatureLower :type Integer))
  (`KismetSystemLibrary.PrintString` "Beat"))

(event `self.FMODAudioScene.OnTimelineMarker`
  (params (Name :type String) (Position :type Integer))
  (`KismetSystemLibrary.PrintString` "Time"))

(fn `InitUI`
  (bind _returnvalue (`|CreateWidget` "/Game/BluePrint/UserUI.UserUI_C"))
  (bind _output_get (set `self.userUI` _returnvalue))
  (set `/Game/BluePrint/UserUI.AudioComp` (`self.FMODAudioScene`) _output_get)
  (`/Game/BluePrint/UserUI.ShowUI` _output_get))

(fn `UserConstructionScript`)