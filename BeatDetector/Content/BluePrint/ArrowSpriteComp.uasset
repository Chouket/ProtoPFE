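; ArrowSpriteComp is a Blueprint, likely for an arrow sprite, that computes a transform moving from a start toward a target.
; Its Update function returns a linear blend of StartTransform and Target at LerpF, then advances LerpF by world delta seconds times Speed.
; The event graph is empty, and Update neither applies the transform nor clamps or resets LerpF.
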(fn `Update`
  (returns (NewParam :type "Transform Structure"))
  (locals (NewPos :type "Transform Structure"))
  (bind _lerpf (`self.LerpF`))
  (bind _output_get (set `local.NewPos` (`KismetMathLibrary.TLerp` (`self.StartTransform`) (`self.Target`) _lerpf)))
  (set `self.LerpF` (+ _lerpf (* (`GameplayStatics.GetWorldDeltaSeconds`) (`self.Speed`))))
  (return _output_get))