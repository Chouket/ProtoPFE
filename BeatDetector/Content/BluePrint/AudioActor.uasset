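; AudioActor is an actor that bootstraps the FMOD audio manager and the player UI when play begins.
; InitAudio constructs a BPAudioManagerFMOD object owned by the actor and initializes it, with an on-screen error message for initialization failure.
; InitUI then creates the PlayerUI widget and hands it a reference back to the actor before BeginPlay shows it.
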(event `self.ReceiveBeginPlay`
  (`self.InitAudio`)
  (`self.InitUI`)
  (`/Game/BluePrint/PlayerUI.ShowUI` (`self.PlayerUI`)))

(fn `InitAudio`
  (bind _returnvalue (`|GenericCreateObject` "/Script/BeatDetector.BPAudioManagerFMOD" self))
  (bind _output_get (set `self.AudioManager` _returnvalue))
  (bind _returnvalue_2 (`BPAudioManagerFMOD.InitializeManager` _output_get))
  (switch `int` _returnvalue_2
    (:`Default`
      (`KismetSystemLibrary.PrintString` "ERROR : AudioManager initialize has failed"))))

(fn `InitUI`
  (bind _returnvalue (`|CreateWidget` "/Game/BluePrint/PlayerUI.PlayerUI_C"))
  (bind _output_get (set `self.PlayerUI` _returnvalue))
  (set `/Game/BluePrint/PlayerUI.GameActor` self _output_get))

(fn `UserConstructionScript`)