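; RythmGame is a Blueprint actor that randomly spawns arrow sprites for a rhythm game.
; Each Tick has a one-in-ten chance to call RandomSpawn, so spawning follows frame rate rather than a beat.
; RandomSpawn picks the left, down, up or right template arrow.
; InstantiateFromArrow adds a Paper Sprite component with that arrow's color and world transform, then offsets it upward along Z.
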(event `self.ReceiveTick`
  (params (DeltaSeconds :type "Float (single-precision)"))
  (if (== (`KismetMathLibrary.RandomIntegerInRange` 1 10) 1)
    (`self.RandomSpawn`)))

(fn `InstantiateFromArrow`
  (params (ArrowRef :type "PaperSpriteComponent Object Reference"))
  (returns (NewArrow :type "PaperSpriteComponent Object Reference"))
  (locals (NewLocalVar_0 :type "PaperSprite Object Reference"))
  (bind _returnvalue (`AddComponent|NODE_AddPaperSpriteComponent-1`))
  (`PaperSpriteComponent.SetSpriteColor` _returnvalue (`PaperSpriteComponent.SpriteColor` ArrowRef))
  (`SceneComponent.K2_SetWorldTransform` _returnvalue (`SceneComponent.K2_GetComponentToWorld` ArrowRef) false false)
  (`SceneComponent.K2_AddWorldOffset` _returnvalue (0.0 0.0 1000.0) false false)
  (return _returnvalue))

(fn `RandomSpawn`
  (locals (newArrow :type "PaperSpriteComponent Object Reference"))
  (switch `int` (`KismetMathLibrary.RandomIntegerInRange` 0 3)
    (:`Default`
      (`KismetSystemLibrary.PrintString` "Error !"))
    (:`0`
      (`self.InstantiateFromArrow` (`self.LeftArrow`)))
    (:`1`
      (`self.InstantiateFromArrow` (`self.DownArrow`)))
    (:`2`
      (`self.InstantiateFromArrow` (`self.UpArrow`)))
    (:`3`
      (`self.InstantiateFromArrow` (`self.RightArrow`)))))

(fn `UserConstructionScript`)